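; Player character with camera look, movement, double jump, a cooldown-limited dash and checkpoint respawning.
; A CanMove counter gates input during dash and death, while a short delay after leaving the ground gives coyote time before removing a jump.
; Dash suspends gravity and braking around a forward launch; damage triggers death effects, a fade and teleport to the latest checkpoint or PlayerStart.
; Footstep events trace under four foot sockets to play sounds.
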(event `self.ReceiveBeginPlay`
  (`self.SetNewJumpCount` 1)
  (set `self.JumpMaxHoldTime` 0.2)
  (set `self.GravityScaleRef` (`CharacterMovementComponent.GravityScale` (`self.CharacterMovement`)))
  (bind _returnvalue (`GameplayStatics.GetActorOfClass` "/Script/Engine.PlayerStart"))
  (set `self.RespawnTransform` (`self.GetTransform` _returnvalue)))

(event `EnhancedInput|/Game/Inputs/IA_Look`
  (params (ActionValue :type "Vector2D Structure") (ElapsedSeconds :type "Float (double-precision)") (TriggeredSeconds :type "Float (double-precision)") (InputAction :type "InputAction Object Reference" :default "/Game/Inputs/IA_Look.IA_Look"))
  (bind (_x _y) (`KismetMathLibrary.BreakVector2D` ActionValue))
  (:`Triggered`
    (`self.CanMoveState`
      (:`Can Move`
        (bind _settingsave (message `/Game/Blueprints/Interfaces/BPI_GameInstance.ReturnSettingsSave` (`GameplayStatics.GetGameInstance`)))
        (bind _sensitivity (`/Game/Blueprints/Core/BP_SettingsSave.Sensitivity` _settingsave))
        (`self.AddControllerYawInput` (* _sensitivity _x (`KismetMathLibrary.SelectFloat` -1.0 1.0 (`/Game/Blueprints/Core/BP_SettingsSave.InvertX` _settingsave))))
        (`self.AddControllerPitchInput` (* _sensitivity _y (`KismetMathLibrary.SelectFloat` -1.0 1.0 (`/Game/Blueprints/Core/BP_SettingsSave.InvertY` _settingsave))))))))

(event `EnhancedInput|/Game/Inputs/IA_Move`
  (params (ActionValue :type "Vector2D Structure") (ElapsedSeconds :type "Float (double-precision)") (TriggeredSeconds :type "Float (double-precision)") (InputAction :type "InputAction Object Reference" :default "/Game/Inputs/IA_Move.IA_Move"))
  (bind (_returnvalue_roll _returnvalue_pitch _returnvalue_yaw) (`KismetMathLibrary.BreakRotator` (`self.GetControlRotation`)))
  (bind (_x _y) (`KismetMathLibrary.BreakVector2D` ActionValue))
  (bind (_returnvalue_roll_2 _returnvalue_pitch_2 _returnvalue_yaw_2) (`KismetMathLibrary.BreakRotator` (`self.GetControlRotation`)))
  (:`Triggered`
    (`self.CanMoveState`
      (:`Can Move`
        (`self.AddMovementInput` (`KismetMathLibrary.GetRightVector` (`KismetMathLibrary.MakeRotator` 0.0 0.0 _returnvalue_yaw)) _x)
        (`self.AddMovementInput` (`KismetMathLibrary.GetForwardVector` (`KismetMathLibrary.MakeRotator` 0.0 0.0 _returnvalue_yaw_2)) _y)))))

(event `EnhancedInput|/Game/Inputs/IA_Jump`
  (params (ActionValue :type Boolean) (ElapsedSeconds :type "Float (double-precision)") (TriggeredSeconds :type "Float (double-precision)") (InputAction :type "InputAction Object Reference" :default "/Game/Inputs/IA_Jump.IA_Jump"))
  (:`Started`
    (`self.CanMoveState`
      (:`Can Move`
        (if (`KismetMathLibrary.Conv_IntToBool` (`self.CurrentJumpCount`))
          (`/Engine/EditorBlueprintResources/StandardMacros.DecrementInt` (`self.CurrentJumpCount`)
            (:`  `
              (`self.Jump`)))))))
  (:`Completed`
    (`self.StopJumping`)))

(event `self.K2_OnMovementModeChanged`
  (params (PrevMovementMode :type "EMovementMode Enum" :default "MOVE_None") (NewMovementMode :type "EMovementMode Enum" :default "MOVE_None") (PrevCustomMode :type Byte) (NewCustomMode :type Byte))
  (if (`NavMovementComponent.IsMovingOnGround` (`self.CharacterMovement`))
    (set `self.CurrentJumpCount` 2)
    (goto _label :!via `Reset`)
    (else
      (`/Engine/EditorBlueprintResources/StandardMacros.DoOnce` false :!label _label
        (:`Completed`
          (`KismetSystemLibrary.RetriggerableDelay` 0.2)
          (if (and (not (`NavMovementComponent.IsMovingOnGround` (`self.CharacterMovement`))) (== (`self.CurrentJumpCount`) (- (`self.JumpMaxCount`) 1)))
            (`/Engine/EditorBlueprintResources/StandardMacros.DecrementInt` (`self.CurrentJumpCount`))))))))

(event `EnhancedInput|/Game/Inputs/IA_Dash`
  (params (ActionValue :type Boolean) (ElapsedSeconds :type "Float (double-precision)") (TriggeredSeconds :type "Float (double-precision)") (InputAction :type "InputAction Object Reference" :default "/Game/Inputs/IA_Dash.IA_Dash"))
  (bind (_returnvalue_roll _returnvalue_pitch _returnvalue_yaw) (`KismetMathLibrary.BreakRotator` (`self.GetControlRotation`)))
  (bind _charactermovement (`self.CharacterMovement`))
  (bind _charactermovement_2 (`self.CharacterMovement`))
  (bind _returnvalue (`KismetMathLibrary.GetForwardVector` (`KismetMathLibrary.MakeRotator` 0.0 0.0 _returnvalue_yaw)))
  (:`Started`
    (`/Game/Blueprints/Libraries/ML_Utils.DoOnceWithAfter` :!label _label_2
      (:`Once`
        (`|PlayMontage` (`self.Mesh`) "/Game/3D/Character/AM_Dash.AM_Dash"
          (:`then`
            (`/Engine/EditorBlueprintResources/StandardMacros.IncrementInt` (`self.CanMove`)
              (:`  `
                (`KismetSystemLibrary.DelayUntilNextTick`)
                (`|ExecutionSequence`
                  (:`then_0`
                    (set `CharacterMovementComponent.GravityScale` 0.0 _charactermovement_2)
                    (set `CharacterMovementComponent.BrakingDecelerationFalling` 0.0 _charactermovement_2)
                    (set `CharacterMovementComponent.BrakingDecelerationWalking` 0.0 _charactermovement_2)
                    (set `MovementComponent.Velocity` (0.0 0.0 0.0) _charactermovement_2)
                    (set `CharacterMovementComponent.RotationRate` (struct :`Yaw` -1.0) _charactermovement_2))
                  (:`then_1`
                    (`self.AddMovementInput` _returnvalue)
                    (`self.LaunchCharacter` (* _returnvalue 1800.0))
                    (`GameplayStatics.PlaySoundAtLocation` "/Game/Audio/MetaSounds/MS_Squeak.MS_Squeak" (`SceneComponent.K2_GetComponentLocation` (`self.Camera`)) (struct) 1.0 1.0 0.0 null null null null)
                    (`ActorComponent.SetActive` (`self.DashEffect`) true true)
                    (`KismetSystemLibrary.Delay` 0.2)
                    (`ActorComponent.SetActive` (`self.DashEffect`) false false))))))
          (:`OnCompleted`
            (`self.bHidden` :!label _label_3
              (:`then`
                _)
              (:`else`
                (set `CharacterMovementComponent.GravityScale` (`self.GravityScaleRef`) (`self.CharacterMovement`))))
            (set `CharacterMovementComponent.BrakingDecelerationFalling` (`self.BrakingDeceleration`) _charactermovement)
            (set `CharacterMovementComponent.BrakingDecelerationWalking` (`self.BrakingDeceleration`) _charactermovement)
            (set `CharacterMovementComponent.RotationRate` (struct :`Yaw` 500.0) _charactermovement)
            (`/Engine/EditorBlueprintResources/StandardMacros.DecrementInt` (`self.CanMove`)
              (:`  `
                (`KismetSystemLibrary.Delay` 3.0)
                (goto _label_2 :!via `Reset`))))
          (:`OnInterrupted`
            (goto _label_3)))))))

(event `self.ReceiveAnyDamage`
  (params (Damage :type "Float (single-precision)") (DamageType :type "DamageType Object Reference") (InstigatedBy :type "Controller Object Reference") (DamageCauser :type "Actor Object Reference"))
  (bind _charactermovement (`self.CharacterMovement`))
  (bind _rotation (.rotation (`self.RespawnTransform`)))
  (`/Engine/EditorBlueprintResources/StandardMacros.IncrementInt` (`self.CanMove`)
    (:`  `
      (`self.SetActorHiddenInGame` true)
      (`KismetSystemLibrary.DelayUntilNextTick`)
      (set `CharacterMovementComponent.GravityScale` 0.0 _charactermovement)
      (set `MovementComponent.Velocity` (0.0 0.0 0.0) _charactermovement)
      (`NiagaraFunctionLibrary.SpawnSystemAtLocation` "/Game/Particles/NS_Death.NS_Death" (`self.K2_GetActorLocation`))
      (`KismetSystemLibrary.Delay` 1.5)
      (`PlayerCameraManager.StartCameraFade` :`self` (`GameplayStatics.GetPlayerCameraManager` 0) :`ToAlpha` 1.0 :`Duration` 1.0 :`bShouldFadeAudio` true :`bHoldWhenFinished` true)
      (`KismetSystemLibrary.Delay` 1.2)
      (`self.K2_SetActorLocationAndRotation` (.location (`self.RespawnTransform`)) _rotation false true)
      (`Controller.SetControlRotation` (`GameplayStatics.GetPlayerController` 0) _rotation)
      (set `CharacterMovementComponent.GravityScale` (`self.GravityScaleRef`) (`self.CharacterMovement`))
      (`self.SetActorHiddenInGame` false)
      (`/Engine/EditorBlueprintResources/StandardMacros.DecrementInt` (`self.CanMove`)
        (:`  `
          (`PlayerCameraManager.StartCameraFade` :`self` (`GameplayStatics.GetPlayerCameraManager` 0) :`FromAlpha` 1.0 :`Duration` 0.5 :`bShouldFadeAudio` true))))))

(event `/Game/Blueprints/Interfaces/BPI_Player.CheckpointReached`
  (params (CheckpointRef :type "/Game/Blueprints/World/BP_Checkpoint Object Reference"))
  (bind _currentcheckpoint (`self.CurrentCheckpoint`)
    (:`then`
      (if (!= _currentcheckpoint CheckpointRef)
        (`/Game/Blueprints/World/BP_Checkpoint.DeactivateCheckpoint` (`self.CurrentCheckpoint`))
        (bind _output_get (set `self.CurrentCheckpoint` CheckpointRef :!label _label_4))
        (set `self.RespawnTransform` (`SceneComponent.K2_GetComponentToWorld` (`/Game/Blueprints/World/BP_Checkpoint.Arrow` _output_get)))))
    (:`else`
      (goto _label_4))))

(event `/Game/Blueprints/Interfaces/BPI_Player.Footstep`
  (params (IsFrontRight :type Boolean) (IsBackRight :type Boolean))
  (bind _returnvalue (`SceneComponent.GetSocketLocation` (`self.Mesh`) (`KismetMathLibrary.SelectName` "BackRightFoot" "BackLeftFoot" IsBackRight)))
  (bind _returnvalue_2 (`SceneComponent.GetSocketLocation` (`self.Mesh`) (`KismetMathLibrary.SelectName` "FrontRightFoot" "FrontLeftFoot" IsFrontRight)))
  (bind (_outhit _returnvalue_3) (`KismetSystemLibrary.LineTraceSingle` _returnvalue_2 (- _returnvalue_2 (0.0 0.0 20.0)) "TraceTypeQuery1"))
  (bind (_outhit_2 _returnvalue_4) (`KismetSystemLibrary.LineTraceSingle` _returnvalue (- _returnvalue (0.0 0.0 20.0)) "TraceTypeQuery1"))
  (if (and _returnvalue_4 _returnvalue_3)
    (`GameplayStatics.SpawnSoundAtLocation` "/Game/Audio/MetaSounds/MS_SoftFootsteps.MS_SoftFootsteps" (`.ImpactPoint` (`GameplayStatics.BreakHitResult` _outhit_2)) (struct) 1.0 1.0 0.0 "/Game/Audio/A_FootstepAttenuation.A_FootstepAttenuation" null)
    (`GameplayStatics.SpawnSoundAtLocation` "/Game/Audio/MetaSounds/MS_SoftFootsteps.MS_SoftFootsteps" (`.ImpactPoint` (`GameplayStatics.BreakHitResult` _outhit)) (struct) 1.0 1.0 0.0 "/Game/Audio/A_FootstepAttenuation.A_FootstepAttenuation" null)))

(fn `SetNewJumpCount`
  (params (NewJumpCount :type Integer))
  (bind _output_get (set `self.CurrentJumpCount` NewJumpCount))
  (set `self.JumpMaxCount` (+ _output_get 1)))

(fn `UserConstructionScript`)