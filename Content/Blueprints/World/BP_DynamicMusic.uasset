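; BP_DynamicMusic plays a MetaSound as 2D music on BeginPlay and raises its intensity through the OverallGain float parameter.
; Each React call plays GainTimeline, feeding its curve value plus CurrentGain into that parameter and incrementing CurrentGain when the timeline finishes forward.
; Calls arriving while the timeline runs retry each tick through a DelayUntilNextTick loop until it is free.
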(event `self.ReceiveBeginPlay`
  (bind _returnvalue (`GameplayStatics.SpawnSound2D` "/Game/Audio/MetaSounds/MS_DynamicMusic.MS_DynamicMusic" 1.0 1.0 0.0 null))
  (set `self.Music` _returnvalue))

(event `/Game/Blueprints/Interfaces/BPI_React.React`
  (if (`TimelineComponent.IsPlaying` (`self.GainTimeline`)) :!label _label
    (`KismetSystemLibrary.DelayUntilNextTick`)
    (goto _label)
    (else
      (bind (_direction _gain) (`Timeline|GainTimeline` :!via `PlayFromStart`)
        (:`Update`
          (`AudioComponent.SetFloatParameter` (`self.Music`) "OverallGain" (+ _gain (`self.CurrentGain`))))
        (:`Finished`
          (switch `ETimelineDirection` _direction
            (:`Forward`
              (`/Engine/EditorBlueprintResources/StandardMacros.IncrementFloat` (`self.CurrentGain`)))))))))

(fn `UserConstructionScript`)