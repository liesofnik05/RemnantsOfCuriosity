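; BP_C_TriggerCollectible is a collectible that triggers a reaction in other actors when it is collected.
; On collect, it sends ReactMessage to ActorToReact if that is not empty, then runs the parent's collect logic.
; BeginPlay is disabled, the construction script only calls the parent, and a DestroyActor call is left unconnected.
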(event `self.OnCollect`
  (`|ExecutionSequence`
    (:`then_0`
      (if (`KismetArrayLibrary.Array_IsNotEmpty` (`self.ActorToReact`))
        (message `/Game/Blueprints/Interfaces/BPI_React.React` (`self.ActorToReact`))))
    (:`then_1`
      (`parent.OnCollect`))))

(fn `UserConstructionScript`
  (`parent.UserConstructionScript`))