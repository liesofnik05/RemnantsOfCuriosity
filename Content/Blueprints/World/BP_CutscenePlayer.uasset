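; BP_CutscenePlayer plays the assigned CutsceneToPlay level sequence when its React event fires.
; React caches the player, binds the sequencer's finished event and starts playback.
; When HasCamera is set, it increments the player's CanMove counter and pushes a CAW_Cutscene widget onto the main UI stack.
; OnFinished removes that widget and decrements the counter again.
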(event `/Game/Blueprints/Interfaces/BPI_React.React`
  (`self.CutsceneToPlay`
    (:`then`
      (`self.PlayOnce`
        (:`then`
          (`/Engine/EditorBlueprintResources/StandardMacros.DoOnce` false
            (:`Completed`
              _)))
        (:`else`
          _))
      (`|ExecutionSequence`
        (:`then_0`
          (`self.PlayerRef`
            (:`then`)
            (:`else`
              (bind _asbp_player (cast `/Game/Blueprints/Core/BP_Player` (`GameplayStatics.GetPlayerCharacter` 0)))
              (set `self.PlayerRef` _asbp_player))))
        (:`then_1`
          (add `MovieSceneSequencePlayer.OnFinished` (`LevelSequenceActor.SequencePlayer` (`self.CutsceneToPlay`)) (`|CreateDelegate` :!event `OnFinished`)))
        (:`then_2`
          (`self.HasCamera`
            (:`then`
              (`/Engine/EditorBlueprintResources/StandardMacros.IncrementInt` (`/Game/Blueprints/Core/BP_Player.CanMove` (`self.PlayerRef`))
                (:`  `
                  (bind _returnvalue (`CommonActivatableWidgetContainerBase.BP_AddWidget` (`/Game/Blueprints/Libraries/FL_Utils.ReturnMainStack` (`GameplayStatics.GetPlayerController` 0)) "/Game/Blueprints/UI/CAW_Cutscene.CAW_Cutscene_C"))
                  (set `self.Widget` _returnvalue))))
            (:`else`)))
        (:`then_3`
          (`MovieSceneSequencePlayer.Play` (`LevelSequenceActor.SequencePlayer` (`self.CutsceneToPlay`))))))
    (:`else`)))

(event `OnFinished`
  (`self.HasCamera`
    (:`then`
      (`CommonActivatableWidgetContainerBase.RemoveWidget` (`/Game/Blueprints/Libraries/FL_Utils.ReturnMainStack` (`GameplayStatics.GetPlayerController` 0)) (`self.Widget`))
      (bind _playerref (`self.PlayerRef`)
        (:`then`
          (`/Engine/EditorBlueprintResources/StandardMacros.DecrementInt` (`/Game/Blueprints/Core/BP_Player.CanMove` _playerref)))
        (:`else`)))
    (:`else`)))

(fn `UserConstructionScript`)