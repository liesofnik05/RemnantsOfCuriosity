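; BP_Checkpoint is a world checkpoint that lights up when the player reaches it.
; A box overlap by BP_Player activates the particle, notifies the player with itself and swaps the cone to a lantern material.
; A DoOnce limits the point light toggle to the first activation.
; DeactivateCheckpoint stops only the particle, leaving the material and light as they are.
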(event `self.Box.OnComponentBeginOverlap`
  (params (OverlappedComponent :type "PrimitiveComponent Object Reference") (OtherActor :type "Actor Object Reference") (OtherComp :type "PrimitiveComponent Object Reference") (OtherBodyIndex :type Integer) (bFromSweep :type Boolean) (SweepResult :type "HitResult Structure (by ref)"))
  (if (== (`GameplayStatics.GetObjectClass` OtherActor) "/Game/Blueprints/Core/BP_Player.BP_Player_C")
    (`ActorComponent.Activate` (`self.Particle`) false)
    (message `/Game/Blueprints/Interfaces/BPI_Player.CheckpointReached` OtherActor self)
    (`PrimitiveComponent.SetMaterial` (`self.Cone`) 0 "/Game/Materials/M_CheckpointLantern.M_CheckpointLantern")
    (`/Engine/EditorBlueprintResources/StandardMacros.DoOnce` false
      (:`Completed`
        (`SceneComponent.ToggleVisibility` (`self.PointLight`) false)))))

(event `DeactivateCheckpoint`
  (`ActorComponent.Deactivate` (`self.Particle`)))

(fn `UserConstructionScript`)