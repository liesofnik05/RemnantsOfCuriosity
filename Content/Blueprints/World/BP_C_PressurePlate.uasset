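; BP_C_PressurePlate is a world pressure plate that sinks when the player steps onto it.
; Box overlap events compare the other actor's class exactly to BP_Player and call MovePlate, which eases the SMPlate mesh to a new relative height.
; Stepping off raises the plate again only if RevertPressedState is set.
; The file shows only this movement, with no signal to other actors.
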(event `self.Box.OnComponentBeginOverlap`
  (params (OverlappedComponent :type "PrimitiveComponent Object Reference") (OtherActor :type "Actor Object Reference") (OtherComp :type "PrimitiveComponent Object Reference") (OtherBodyIndex :type Integer) (bFromSweep :type Boolean) (SweepResult :type "HitResult Structure (by ref)"))
  (if (== (`GameplayStatics.GetObjectClass` OtherActor) "/Game/Blueprints/Core/BP_Player.BP_Player_C")
    (`self.MovePlate` 2.0)))

(event `self.Box.OnComponentEndOverlap`
  (params (OverlappedComponent :type "PrimitiveComponent Object Reference") (OtherActor :type "Actor Object Reference") (OtherComp :type "PrimitiveComponent Object Reference") (OtherBodyIndex :type Integer))
  (if (and (== (`GameplayStatics.GetObjectClass` OtherActor) "/Game/Blueprints/Core/BP_Player.BP_Player_C") (`self.RevertPressedState`))
    (`self.MovePlate` 10.0)))

(event `MovePlate`
  (params (Z :type "Float (double-precision)"))
  (`KismetSystemLibrary.MoveComponentTo` (`self.SM_Plate`) (`KismetMathLibrary.MakeVector` 0.0 0.0 Z) (struct) true true 0.5))

(fn `UserConstructionScript`
  (`parent.UserConstructionScript`))