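; Collectible pickup that flies to the player on overlap and adds its value through the game mode.
; An idle timeline started on BeginPlay spins and bobs the Scene component.
; The first BP_Player overlap starts a collect timeline that lerps the actor toward a point below the player's origin.
; Once close enough, it sends its Value to the game mode by interface message and destroys itself.
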(event `self.ReceiveBeginPlay`
  (`TimelineComponent.Play` (`self.IdleTimeline`)))

(event `self.Sphere.OnComponentBeginOverlap`
  (params (OverlappedComponent :type "PrimitiveComponent Object Reference") (OtherActor :type "Actor Object Reference") (OtherComp :type "PrimitiveComponent Object Reference") (OtherBodyIndex :type Integer) (bFromSweep :type Boolean) (SweepResult :type "HitResult Structure (by ref)"))
  (if (== (`GameplayStatics.GetObjectClass` OtherActor) "/Game/Blueprints/Core/BP_Player.BP_Player_C")
    (set `self.HitActor` OtherActor)
    (`/Engine/EditorBlueprintResources/StandardMacros.DoOnce` false
      (:`Completed`
        (bind (_direction _value) (`Timeline|CollectTimeline`)
          (:`Update`
            (bind _hitactor (`self.HitActor`)
              (:`then`
                (`self.K2_SetActorLocation` (`KismetMathLibrary.VLerp` (`self.K2_GetActorLocation`) (- (`self.K2_GetActorLocation` _hitactor) (0.0 0.0 90.0)) _value) true)
                (if (== (`self.K2_GetActorLocation`) (- (`self.K2_GetActorLocation` (`self.HitActor`)) (0.0 0.0 90.0)) :`ErrorTolerance` 20.0)
                  (`self.OnCollect`)))
              (:`else`))))))))

(event `OnCollect`
  (message `/Game/Blueprints/Interfaces/BPI_GameMode.IncreaseCollectibleValue` (`GameplayStatics.GetGameMode`) (`self.Value`))
  (`self.K2_DestroyActor`))

(fn `UserConstructionScript`)