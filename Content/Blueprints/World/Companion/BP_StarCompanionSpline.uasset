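; A glowing star companion that travels along a spline, pacing itself to the player's distance.
; On BeginPlay a timeline starts, moving and rotating the scene component along the spline while an attached sparkle sound plays.
; Each update scales the timeline play rate by Speed and a clamped distance mapping, so the star moves faster when the player is near and slows as they fall behind.
; A point light follows the star mesh.
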(event `self.ReceiveBeginPlay`
  (bind _spline (`self.Spline`))
  (`/Engine/EditorBlueprintResources/StandardMacros.IsValid` (`GameplayStatics.GetPlayerCharacter` 0)
    (:`Is Valid`
      (`TimelineComponent.SetPlayRate` (`self.MoveTimeline`) 0.0)
      (`GameplayStatics.SpawnSoundAttached` (`self.MovementSound`) (`self.StaticMesh`) "None" (0.0 0.0 0.0) (struct) "KeepRelativeOffset" false 0.25 1.0 0.0 "/Game/Audio/A_SparklesAttenuation.A_SparklesAttenuation" null)
      (bind (_direction _value) (`Timeline|MoveTimeline`)
        (:`Update`
          (bind _returnvalue (`KismetMathLibrary.Lerp` 0.0 (`SplineComponent.GetSplineLength` _spline) _value))
          (`SceneComponent.K2_SetWorldLocation` (`self.Scene`) (`SplineComponent.GetLocationAtDistanceAlongSpline` _spline _returnvalue "World") true false)
          (`SceneComponent.K2_SetWorldRotation` (`self.Scene`) (`SplineComponent.GetRotationAtDistanceAlongSpline` (`self.Spline`) _returnvalue "World") true false)
          (`TimelineComponent.SetPlayRate` (`self.MoveTimeline`) (* (`self.Speed`) (`KismetMathLibrary.MapRangeClamped` (`KismetMathLibrary.VSize` (- (`SceneComponent.K2_GetComponentLocation` (`self.StaticMesh`)) (`self.K2_GetActorLocation` (`GameplayStatics.GetPlayerCharacter` 0)))) 0.0 1000.0 3.0)))
          (`SceneComponent.K2_SetWorldLocation` (`self.PointLight`) (`SceneComponent.K2_GetComponentLocation` (`self.StaticMesh`)) true false)
          (`SceneComponent.K2_SetWorldRotation` (`self.PointLight`) (`SceneComponent.K2_GetComponentRotation` (`self.StaticMesh`)) true false))))))

(fn `UserConstructionScript`)