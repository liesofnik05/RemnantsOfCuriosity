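; BP_Goal is the level goal that ends play by showing the outro screen when its React event fires.
; React pauses the game, shows the mouse cursor, switches to UI-only input and adds CAW_Outro to the player's main widget stack.
; A disconnected leftover path would instead wait an optional delay, flag the credits message on the GameInstance and open the first level.
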(event `/Game/Blueprints/Interfaces/BPI_React.React`
  (`GameplayStatics.SetGamePaused` true)
  (set `PlayerController.bShowMouseCursor` true (`GameplayStatics.GetPlayerController` 0))
  (`WidgetBlueprintLibrary.SetInputMode_UIOnlyEx` (`GameplayStatics.GetPlayerController` 0) null)
  (`CommonActivatableWidgetContainerBase.BP_AddWidget` (`/Game/Blueprints/Libraries/FL_Utils.ReturnMainStack` (`GameplayStatics.GetPlayerController` 0)) "/Game/Blueprints/UI/CAW_Outro.CAW_Outro_C"))

(fn `UserConstructionScript`)